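; AI controller for lane creeps that runs BT_Creep on possession and destroys itself on unpossess.
; Tick advances the creep along Line waypoints, writing the current location to the Blackboard.
; Perception tracks visible BPI_Attackable actors, from which Tick writes the nearest as target, plus an attack-range flag.
; The IsMyTeam filter has its tag check unconnected, and the custom closest-attackable search is never called.
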(event OnTargetPerceptionUpdated(AIPerception)
  (params (Actor :type Actor%20Object%20Reference) (Stimulus :type AI%20Stimulus%20Structure))
  (if (Utilities|DoesObjectImplementInterface Actor "/Game/Creeps/BPI_Attackable.BPI_Attackable_C")
    (if (not (Utilities|IsMyTeam Actor))
      (if (.bSuccessfullySensed (Utilities|Struct|BreakAIStimulus Stimulus))
        (Utilities|Array|AddUnique (Variables|Default|GetAttackables%20In%20View) Actor)
        (else
          (Utilities|Array|RemoveItem (Variables|Default|GetAttackables%20In%20View) Actor))))))

(event EventTick
  (params (DeltaSeconds :type Float%20%28single-precision%29))
  (bind _creep (Variables|Default|GetCreep))
  (bind _attackables_in_view (Variables|Default|GetAttackables%20In%20View))
  (bind _creep_2 (Variables|Default|GetCreep))
  (bind _returnvalue (Transformation|GetActorLocation _creep_2))
  (bind _attack_range (Variables|/Game/Creeps/BP_Creep.BP_Creep_C|GetAttack%20Range _creep))
  (bind (_distance _returnvalue_2) (Actor|FindNearestActor _returnvalue _attackables_in_view))
  (bind _returnvalue_3 (< _distance _attack_range))
  (CallFunction|CheckandResolveLineAdvancement)
  (Utilities|IsValid _returnvalue_2
    (:Is%20Valid
      (Utilities|SetCurrentTargetinBB _returnvalue_2)
      (Development|PrintString (Utilities|String|ToString(Boolean) _returnvalue_3))
      (Utilities|SetIsTargetinFightRangeinBB _returnvalue_3))))

(event EventPossess
  (params (PossessedPawn :type Pawn%20Object%20Reference))
  (bind _asbp_creep (Utilities|Casting|CastToBP_Creep PossessedPawn))
  (Variables|Default|SetCreep _asbp_creep)
  (AI|RunBehaviorTree "/Game/Creeps/BT_Creep.BT_Creep")
  (CallFunction|SetCurrentLineWaypointbyIndex))

(event EventUnPossess
  (params (UnpossessedPawn :type Pawn%20Object%20Reference))
  (Actor|DestroyActor))

(fn ConstructionScript)

(fn FindClosestAttackableinViewandRemoveNotValid
  (bind _attackables_in_view (Variables|Default|GetAttackables%20In%20View))
  (bind _output (Utilities|Array|Get(acopy) _attackables_in_view))
  ;[0.15 0.15 0.15 0.5] Set first as the current closest
  (LocalVariables|SetCurrent%20Closest%20Distance%20Squared (Transformation|GetSquaredDistanceTo _output))
  (LocalVariables|SetCurrent%20Closest _output)
  (for _array_element (Variables|Default|GetAttackables%20In%20View)
    (Utilities|IsValid _array_element
      (:Is%20Valid
        ;[0.15 0.15 0.15 0.5] If closer: update closest
        (if (< (Transformation|GetSquaredDistanceTo (Variables|Default|GetCreep) _array_element) (LocalVariables|GetCurrent%20Closest%20Distance%20Squared))
          (LocalVariables|SetCurrent%20Closest _array_element)
          (LocalVariables|SetCurrent%20Closest%20Distance%20Squared (Transformation|GetSquaredDistanceTo (Variables|Default|GetCreep) _array_element))))))
  (return (LocalVariables|GetCurrent%20Closest) (LocalVariables|GetCurrent%20Closest%20Distance%20Squared)))

(fn SetCurrentLineWaypointbyIndex
  (params (New%20Line%20Waypoint%20Idx :type Integer))
  (bind _output_get (Variables|Default|SetCurrent%20Line%20Waypoint%20Idx New%20Line%20Waypoint%20Idx))
  (bind _output_get_2 (Variables|Default|SetCurrent%20Line%20Waypoint (Utilities|Array|Get(acopy) (Utilities|Struct|BreakF_CreepLine (Variables|Default|GetLine)) _output_get)))
  (AI|Components|Blackboard|SetValueasVector (AI|GetBlackboard 0) (Variables|Default|GetCurrent%20Line%20Waypoint%20BB%20Key) (Transformation|GetActorLocation _output_get_2)))

(fn CheckandResolveLineAdvancement
  (if (not (== (Variables|Default|GetCurrent%20Line%20Waypoint%20Idx) (Utilities|Array|LastIndex (Utilities|Struct|BreakF_CreepLine (Variables|Default|GetLine)))))
    (if (Default|HasActorReached (Variables|Default|GetCurrent%20Line%20Waypoint) (Variables|Default|GetCreep))
      (CallFunction|SetCurrentLineWaypointbyIndex (+ (Variables|Default|GetCurrent%20Line%20Waypoint%20Idx) 1)))))